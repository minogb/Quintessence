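; Quint player controller Blueprint that puts the game's user interface on screen.
; On BeginPlay, it checks that it is the local player controller, then creates a UserInterface widget owned by itself and adds it to the viewport.
; An unexecuted branch holds a similar widget setup with no class set, followed by a debug print of a class display name.
; The construction script is empty.
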(event EventBeginPlay
  (if (Pawn|IsLocalPlayerController)
    (bind _returnvalue (UserInterface|CreateWidget "/Game/UserInterface/InventoryUI/UserInterface.UserInterface_C" self))
    (UserInterface|Viewport|AddtoViewport _returnvalue 0)))

(fn ConstructionScript)