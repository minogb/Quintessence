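; NodeBp is a node actor that shows the local player whether their avatar appears in its harvester list.
; Every Tick, SetMesh gets the avatar from the local Quint_PC_BP controller and compares it to each harvester's Player.
; A match sets the static mesh to the inactive material, otherwise to the active one, so the look is specific to each local player.
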(event EventBeginPlay)

(event Collision|EventActorBeginOverlap
  (params (OtherActor :type Actor%20Object%20Reference)))

(event EventTick
  (params (DeltaSeconds :type Float%20%28single-precision%29))
  (CallFunction|SetMesh))

(fn ConstructionScript)

(fn SetMesh
  (bind _returnvalue (Game|GetPlayerController 0))
  (Utilities|IsValid _returnvalue
    (:Is%20Valid
      (if (Pawn|IsLocalPlayerController _returnvalue)
        (bind _asquint_pc_bp (Utilities|Casting|CastToQuint_PC_BP _returnvalue))
        (for _array_element (Class|ResourceNode|GetHarvesters)
          (if (== (Class|QuintPlayerController|GetPlayerAvatar _asquint_pc_bp) (.Player (Utilities|Struct|BreakPlayerHarvestedStruct _array_element)))
            (Rendering|Material|SetMaterial (Variables|Default|GetStaticMesh) 0 (Variables|Default|GetInactiveMaterial))
            (return)))
        (Rendering|Material|SetMaterial (Variables|Default|GetStaticMesh) 0 (Variables|Default|GetActiveMaterial))))))